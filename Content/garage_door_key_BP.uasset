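; Garage door key pickup that the player collects by pressing Interact while standing inside its Box trigger.
; Box overlap with a ThirdPersonCharacter caches the character, enables input for player 0 and opens a Gate; leaving disables input and closes it.
; Pressing Interact through the open gate increments the character's NumKeys, destroys the key actor and prints the new count.
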(event OnComponentBeginOverlap(Box)
  (params (OverlappedComponent :type Primitive%20Component%20Object%20Reference) (OtherActor :type Actor%20Object%20Reference) (OtherComp :type Primitive%20Component%20Object%20Reference) (OtherBodyIndex :type Integer) (bFromSweep :type Boolean) (SweepResult :type Hit%20Result%20Structure%20%28by%20ref%29))
  ;[1 1 1] add +1 to NumKeys variable on pickup, and destroy actor
  (bind _asthird_person_character (Utilities|Casting|CastToThirdPersonCharacter OtherActor))
  (Input|EnableInput (Game|GetPlayerController 0))
  (Utilities|FlowControl|Gate true) ; enters at Open
)

(event OnComponentEndOverlap(Box)
  (params (OverlappedComponent :type Primitive%20Component%20Object%20Reference) (OtherActor :type Actor%20Object%20Reference) (OtherComp :type Primitive%20Component%20Object%20Reference) (OtherBodyIndex :type Integer))
  ;[1 1 1] add +1 to NumKeys variable on pickup, and destroy actor
  (Utilities|Casting|CastToThirdPersonCharacter OtherActor)
  (Input|DisableInput (Game|GetPlayerController 0))
  (Utilities|FlowControl|Gate true) ; enters at Close
)

(event Input|ActionEvents|InputActionInteract
  (params (Key :type Key%20Structure :default "None"))
  ;[1 1 1] add +1 to NumKeys variable on pickup, and destroy actor
  (:Pressed
    (Utilities|FlowControl|Gate true
      (:Exit
        (bind _output_get (Variables|/Game/ThirdPersonBP/Blueprints/ThirdPersonCharacter.ThirdPersonCharacter_C|SetNumKeys (stale OnComponentBeginOverlap(Box) _asthird_person_character) (+ (Variables|/Game/ThirdPersonBP/Blueprints/ThirdPersonCharacter.ThirdPersonCharacter_C|GetNumKeys (stale OnComponentBeginOverlap(Box) _asthird_person_character)) 1)))
        (Actor|DestroyActor)
        (Development|PrintString (Utilities|String|ToString(Integer) _output_get))))))

(fn ConstructionScript)